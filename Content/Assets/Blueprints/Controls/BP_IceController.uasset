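; Player-controlled actor for a grid-based ice-sliding puzzle, turning and sliding with WASD and resetting to its start spot with R.
; StartSlide rejects repeats of the last direction, then the self-calling Slide event makes delayed, swept CubeSize steps until an overlap stops it.
; A HasCollided flag can absorb the next slide request after an overlap.
; Debug keys call BP_AGrid and BP_IceGenerator to show paths, regenerate levels, write level data and print open spots.
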(event Custom|Slide
  (params (Direction :type Vector))
  (if (Variables|Default|GetIsSliding)
    (Transformation|SetActorLocation (+ (Transformation|GetActorLocation) (* Direction (Variables|Default|GetCubeSize))) true false)
    (if (Variables|Default|GetIsSliding)
      (Utilities|FlowControl|Delay 0.1)
      (CallFunction|Slide Direction)
      (else
        (Variables|Default|SetHasCollided false)))))

(event EventBeginPlay
  (Utilities|FlowControl|DelayUntilNextTick)
  (if (Variables|Default|GetHasCollided)
    (Variables|Default|SetHasCollided false)
    (Variables|Default|SetLastSlide "0.000000,1.000000,0.000000")))

(event Collision|EventActorBeginOverlap
  (params (OtherActor :type Actor%20Object%20Reference))
  (Variables|Default|SetIsSliding false)
  (Variables|Default|SetHasCollided true))

(event EventTick
  (params (DeltaSeconds :type Float%20%28single-precision%29)))

(event Input|KeyboardEvents|W
  (params (Key :type Key%20Structure :default "None"))
  (:Pressed
    (if (not (Variables|Default|GetIsSliding))
      (Transformation|SetActorRotation "0.000000,270.000000,0.000000")
      (CallFunction|StartSlide "1.000000,0.000000,0.000000"))))

(event Input|KeyboardEvents|A
  (params (Key :type Key%20Structure :default "None"))
  (:Pressed
    (if (not (Variables|Default|GetIsSliding))
      (Transformation|SetActorRotation "0.000000,180.000000,0.000000")
      (CallFunction|StartSlide "0.000000,-1.000000,0.000000"))))

(event Input|KeyboardEvents|S
  (params (Key :type Key%20Structure :default "None"))
  (:Pressed
    (if (not (Variables|Default|GetIsSliding))
      (Transformation|SetActorRotation "0.000000,90.000000,0.000000")
      (CallFunction|StartSlide "-1.000000,0.000000,0.000000"))))

(event Input|KeyboardEvents|D
  (params (Key :type Key%20Structure :default "None"))
  (:Pressed
    (if (not (Variables|Default|GetIsSliding))
      (Transformation|SetActorRotation "0, 0, 0")
      (CallFunction|StartSlide "0.000000,1.000000,0.000000"))))

(event Input|KeyboardEvents|P
  (params (Key :type Key%20Structure :default "None"))
  (:Pressed
    (bind _returnvalue (Actor|GetActorOfClass "/Game/Assets/Blueprints/Tools/BP_AGrid.BP_AGrid_C"))
    (Default|ShowPath _returnvalue)))

(event Input|KeyboardEvents|R
  (params (Key :type Key%20Structure :default "None"))
  (:Pressed
    (CallFunction|ResetPosition)))

(event Input|KeyboardEvents|G
  (params (Key :type Key%20Structure :default "None"))
  (:Pressed
    (bind _returnvalue (Actor|GetActorOfClass "/Game/Assets/Blueprints/Tools/BP_AGrid.BP_AGrid_C"))
    (Default|ClearGrid _returnvalue)
    (bind _returnvalue_2 (Actor|GetActorOfClass "/Game/Assets/Blueprints/Controls/BP_IceGenerator.BP_IceGenerator_C"))
    (Default|MakeLevel _returnvalue_2)))

(event Input|KeyboardEvents|F
  (params (Key :type Key%20Structure :default "None"))
  (:Pressed
    (bind _returnvalue (Actor|GetActorOfClass "/Game/Assets/Blueprints/Tools/BP_AGrid.BP_AGrid_C"))
    (Default|WriteLevelData _returnvalue)))

(event Input|KeyboardEvents|Down
  (params (Key :type Key%20Structure :default "None"))
  (:Pressed
    (bind _returnvalue (Actor|GetActorOfClass "/Game/Assets/Blueprints/Tools/BP_AGrid.BP_AGrid_C"))
    (bind _openspots (Default|GetOpenSpots _returnvalue 10 5 "-1.000000,0.000000,0.000000"))
    (Development|PrintString (Utilities|String|ToString(Integer) _openspots))))

(fn ConstructionScript)

(fn StartSlide
  (params (Direction :type Vector))
  (if (not (Class|KismetMathLibrary|EqualExactlyVectorVector (Variables|Default|GetLastSlide) Direction))
    (if (Variables|Default|GetHasCollided)
      (Variables|Default|SetHasCollided false)
      (Variables|Default|SetLastSlide Direction)
      (else
        (Variables|Default|SetLastSlide Direction)
        (Variables|Default|SetIsSliding true)
        (CallFunction|Slide Direction)))))

(fn TestCast
  (Development|PrintString "CAST SUCCESS"))

(fn CheckLastSlide
  (params (Direction :type Vector))
  (return (Class|KismetMathLibrary|EqualExactlyVectorVector Direction (Variables|Default|GetLastSlide))))

(fn ResetPosition
  (Variables|Default|SetIsSliding false)
  (Variables|Default|SetHasCollided false)
  (Transformation|SetActorTransform (Math|Transform|MakeTransform (Variables|Default|GetStartSpot)))
  (if (Variables|Default|GetHasCollided)
    (Variables|Default|SetHasCollided false)
    (Variables|Default|SetLastSlide "0.000000,1.000000,0.000000")
    (else
      (Variables|Default|SetLastSlide "-1.000000,-1.000000,-1.000000"))))