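; BP_IceGenerator procedurally builds an ice puzzle level on the BP_AGrid at BeginPlay by walking a cube along a random path.
; The walk moves down, then alternates axes with random direction and length within the open spots, painting cells and placing an obstacle behind each turn.
; It then adds walls and random cubes, makes its end cell BP_IceController's start, and hides itself.
; Debug keys step the walk manually or print open spots.
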(event EventBeginPlay
  (bind _returnvalue (Actor|GetActorOfClass "/Game/Assets/Blueprints/Tools/BP_AGrid.BP_AGrid_C"))
  (Variables|Default|SetGridHolder _returnvalue)
  (CallFunction|MakeLevel))

(event Collision|EventActorBeginOverlap
  (params (OtherActor :type Actor%20Object%20Reference)))

(event EventTick
  (params (DeltaSeconds :type Float%20%28single-precision%29)))

(event Input|KeyboardEvents|W
  (params (Key :type Key%20Structure :default "None"))
  (:Pressed
    (CallFunction|Move "1.000000,0.000000,0.000000")))

(event Input|KeyboardEvents|A
  (params (Key :type Key%20Structure :default "None"))
  (:Pressed
    (CallFunction|Move "0.000000,-1.000000,0.000000")))

(event Input|KeyboardEvents|S
  (params (Key :type Key%20Structure :default "None"))
  (:Pressed
    (CallFunction|Move "-1.000000,0.000000,0.000000")))

(event Input|KeyboardEvents|D
  (params (Key :type Key%20Structure :default "None"))
  (:Pressed
    (CallFunction|Move "0.000000,1.000000,0.000000")))

(event Input|KeyboardEvents|P
  (params (Key :type Key%20Structure :default "None"))
  (:Pressed
    (CallFunction|GenerateDirection)))

(event Input|KeyboardEvents|Left
  (params (Key :type Key%20Structure :default "None"))
  (:Pressed
    (bind _openspots (Default|GetOpenSpots (Variables|Default|GetGridHolder) (Math|Float|Truncate (Variables|Default|GetCurrentRow)) (Math|Float|Truncate (Variables|Default|GetCurrentColumn)) "0.000000,-1.000000,0.000000"))
    (Development|PrintString (Utilities|String|ToString(Integer) _openspots))))

(event Input|KeyboardEvents|Right
  (params (Key :type Key%20Structure :default "None"))
  (:Pressed
    (bind _openspots (Default|GetOpenSpots (Variables|Default|GetGridHolder) (Math|Float|Truncate (Variables|Default|GetCurrentRow)) (Math|Float|Truncate (Variables|Default|GetCurrentColumn)) "0.000000,1.000000,0.000000"))
    (Development|PrintString (Utilities|String|ToString(Integer) _openspots))))

(event Input|KeyboardEvents|Up
  (params (Key :type Key%20Structure :default "None"))
  (:Pressed
    (bind _openspots (Default|GetOpenSpots (Variables|Default|GetGridHolder) (Math|Float|Truncate (Variables|Default|GetCurrentRow)) (Math|Float|Truncate (Variables|Default|GetCurrentColumn)) "1.000000,0.000000,0.000000"))
    (Development|PrintString (Utilities|String|ToString(Integer) _openspots))))

(event Input|KeyboardEvents|Down
  (params (Key :type Key%20Structure :default "None"))
  (:Pressed
    (bind _openspots (Default|GetOpenSpots (Variables|Default|GetGridHolder) (Math|Float|Truncate (Variables|Default|GetCurrentRow)) (Math|Float|Truncate (Variables|Default|GetCurrentColumn)) "-1.000000,0.000000,0.000000"))
    (Development|PrintString (Utilities|String|ToString(Integer) _openspots))))

(event Input|KeyboardEvents|G
  (params (Key :type Key%20Structure :default "None"))
  (:Pressed
    (Default|AddRandomCubes (Variables|Default|GetGridHolder))))

(fn ConstructionScript)

(fn Move
  (params (Direction :type Vector))
  (bind (_x _y) (Math|Vector|BreakVector Direction))
  (CallFunction|CheckAddObstacle Direction)
  (Transformation|SetActorLocation (+ (Transformation|GetActorLocation) (* (Variables|Default|GetCubeSize) Direction)) false false)
  (bind (_row _column) (CallFunction|GetRowColumn))
  (Default|PaintBlock (Variables|Default|GetGridHolder) _row _column)
  (Variables|Default|SetCurrentRow (+ (Variables|Default|GetCurrentRow) _x))
  (Variables|Default|SetCurrentColumn (+ (Variables|Default|GetCurrentColumn) _y)))

(fn GetRowColumn
  (return (Math|Float|Truncate (Variables|Default|GetCurrentRow)) (Math|Float|Truncate (Variables|Default|GetCurrentColumn))))

(fn CheckAddObstacle
  (params (Direction :type Vector))
  (bind (_x _y) (Class|KismetMathLibrary|BreakVector3f Direction))
  (if (not (Class|KismetMathLibrary|EqualExactlyVectorVector (Variables|Default|GetLastMove) Direction))
    (bind (_row _column) (CallFunction|GetRowColumn))
    (Default|AddObstacle (Variables|Default|GetGridHolder) (- _row (Math|Float|Truncate _x)) (- _column (Math|Float|Truncate _y)))
    (Default|PaintBlock (Variables|Default|GetGridHolder) (- _row (Math|Float|Truncate _x)) (- _column (Math|Float|Truncate _y)))
    (Variables|Default|SetLastMove Direction)))

(fn GenerateDirection
  (bind _output_get (Variables|Default|SetDirectionBit (not (Variables|Default|GetDirectionBit))))
  (if _output_get
    (if (Math|Random|RandomBool)
      (bind (_openspots _dir) (Default|GetOpenSpots (Variables|Default|GetGridHolder) (Math|Float|Truncate (Variables|Default|GetCurrentRow)) (Math|Float|Truncate (Variables|Default|GetCurrentColumn)) "1.000000,0.000000,0.000000"))
      (for _index (range 1 (Math|Random|RandomIntegerinRange (/ _openspots 2) _openspots))
        (CallFunction|Move _dir))
      (else
        (bind (_openspots_2 _dir_2) (Default|GetOpenSpots (Variables|Default|GetGridHolder) (Math|Float|Truncate (Variables|Default|GetCurrentRow)) (Math|Float|Truncate (Variables|Default|GetCurrentColumn)) "-1.000000,0.000000,0.000000"))
        (for _index_2 (range 1 (Math|Random|RandomIntegerinRange (/ _openspots_2 2) _openspots_2))
          (CallFunction|Move _dir_2))))
    (elif (Math|Random|RandomBool)
      (bind (_openspots_3 _dir_3) (Default|GetOpenSpots (Variables|Default|GetGridHolder) (Math|Float|Truncate (Variables|Default|GetCurrentRow)) (Math|Float|Truncate (Variables|Default|GetCurrentColumn)) "0.000000,-1.000000,0.000000"))
      (for _index_3 (range 1 (Math|Random|RandomIntegerinRange (/ _openspots_3 2) _openspots_3))
        (CallFunction|Move _dir_3))
      (else
        (bind (_openspots_4 _dir_4) (Default|GetOpenSpots (Variables|Default|GetGridHolder) (Math|Float|Truncate (Variables|Default|GetCurrentRow)) (Math|Float|Truncate (Variables|Default|GetCurrentColumn)) "-0.000000,1.000000,0.000000"))
        (for _index_4 (range 1 (Math|Random|RandomIntegerinRange (/ _openspots_4 2) _openspots_4))
          (CallFunction|Move _dir_4))))))

(fn MakeLevel
  (bind _returnvalue (Transformation|GetActorLocation))
  (CallFunction|GoDown)
  (for _index (range 0 40)
    (CallFunction|GenerateDirection))
  (Default|AddWalls (Variables|Default|GetGridHolder))
  (bind _returnvalue_2 (Actor|GetActorOfClass "/Game/Assets/Blueprints/Controls/BP_IceController.BP_IceController_C"))
  (Transformation|SetActorLocation _returnvalue_2 _returnvalue false false)
  (Variables|/Game/Assets/Blueprints/Controls/BP_IceController.BP_IceController_C|SetStartSpot _returnvalue_2 _returnvalue)
  (Default|PaintBlock (Variables|Default|GetGridHolder) (Math|Float|Truncate (Variables|Default|GetCurrentRow)) (Math|Float|Truncate (Variables|Default|GetCurrentColumn)))
  (Default|AddRandomCubes (Variables|Default|GetGridHolder))
  (Rendering|ToggleVisibility (Variables|Default|GetCube) false))

(fn GoDown
  (bind (_openspots _dir) (Default|GetOpenSpots (Variables|Default|GetGridHolder) (Math|Float|Truncate (Variables|Default|GetCurrentRow)) (Math|Float|Truncate (Variables|Default|GetCurrentColumn)) "-1.000000,0.000000,0.000000"))
  (for _index (range 1 (Math|Random|RandomIntegerinRange (/ _openspots 2) _openspots))
    (CallFunction|Move _dir)))

(fn ResetPosition
  (bind _gridholder (Variables|Default|GetGridHolder))
  (bind _gridholder_2 (Variables|Default|GetGridHolder))
  (bind _numcolumns (Variables|/Game/Assets/Blueprints/Tools/BP_AGrid.BP_AGrid_C|GetNumColumns _gridholder_2))
  (bind _numrows (Variables|/Game/Assets/Blueprints/Tools/BP_AGrid.BP_AGrid_C|GetNumRows _gridholder))
  (bind _returnvalue (/ _numcolumns 2))
  (Transformation|SetActorLocation (Math|Vector|MakeVector (* _numrows (Variables|Default|GetCubeSize)) (* _returnvalue (Variables|Default|GetCubeSize)) (Variables|Default|GetCubeSize)) false false)
  (Variables|Default|SetCurrentRow (Math|Conversions|ToFloat(Integer) _numrows))
  (Variables|Default|SetCurrentColumn (Math|Conversions|ToFloat(Integer) _returnvalue)))