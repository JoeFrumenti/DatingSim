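; BP_AGrid spawns a grid of BP_AGridPiece actors at BeginPlay and positions the BP_IceGenerator at the last row's middle column.
; Pieces live in a flat row-major array that helpers index to paint blocks, reveal obstacle walls or apply brick materials.
; GetOpenSpots steps along a direction counting cells until a painted one, with IsPainted treating out-of-bounds cells as painted.
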(event EventBeginPlay
  (CallFunction|SpawnGrid (Variables|Default|GetNumRows) (Variables|Default|GetNumColumns)))

(fn ConstructionScript)

(fn SpawnGrid
  (params (Rows :type Integer) (Columns :type Integer))
  (bind _returnvalue (/ Rows 1))
  (bind _returnvalue_2 (/ Columns 2))
  (bind _cubesize (Variables|Default|GetCubeSize))
  (for _index (range 1 Rows)
    (for _index_2 (range 1 Columns)
      (bind _returnvalue_3 (Game|SpawnActorfromClass "/Game/Assets/Blueprints/Actors/BP_AGridPiece.BP_AGridPiece_C" (Math|Transform|MakeTransform (Math|Vector|MakeVector (* _index _cubesize) (* _index_2 _cubesize) 0.0)) "Undefined" 0 0))
      (Utilities|Array|Add (Variables|Default|GetGrid) _returnvalue_3))
    (bind _returnvalue_4 (Actor|GetActorOfClass "/Game/Assets/Blueprints/Controls/BP_IceGenerator.BP_IceGenerator_C"))
    (Transformation|SetActorLocation _returnvalue_4 (Math|Vector|MakeVector (Math|Conversions|ToFloat(Integer) (* (Variables|Default|GetCubeSize) _returnvalue)) (Math|Conversions|ToFloat(Integer) (* _returnvalue_2 (Variables|Default|GetCubeSize))) 1e+02) false false)
    (Variables|/Game/Assets/Blueprints/Controls/BP_IceGenerator.BP_IceGenerator_C|SetCurrentColumn _returnvalue_4 (- (Math|Conversions|ToFloat(Integer) _returnvalue_2) 1.0))
    (Variables|/Game/Assets/Blueprints/Controls/BP_IceGenerator.BP_IceGenerator_C|SetCurrentRow _returnvalue_4 (- (Math|Conversions|ToFloat(Integer) _returnvalue) 1.0))))

(fn MakeBrick
  (for _array_element (Variables|Default|GetGrid)
    (Rendering|Material|SetMaterial (Variables|/Game/Assets/Blueprints/Actors/BP_AGridPiece.BP_AGridPiece_C|GetCube _array_element) 0 "/Game/StarterContent/Materials/M_Brick_Clay_New.M_Brick_Clay_New"))
  (Rendering|Material|SetMaterial (Variables|/Game/Assets/Blueprints/Actors/BP_AGridPiece.BP_AGridPiece_C|GetCube (Utilities|Array|Get(acopy) (Variables|Default|GetGrid))) 0 "/Game/StarterContent/Materials/M_AssetPlatform.M_AssetPlatform")
  (Rendering|Material|SetMaterial (Variables|/Game/Assets/Blueprints/Actors/BP_AGridPiece.BP_AGridPiece_C|GetCube (Utilities|Array|Get(acopy) (Variables|Default|GetGrid) 1)) 0 "/Game/StarterContent/Materials/M_AssetPlatform.M_AssetPlatform"))

(fn PaintBlock
  (params (Row :type Integer) (Column :type Integer))
  (bind _index (CallFunction|RowColumntoIndex Row Column))
  (Rendering|Material|SetMaterial (Variables|/Game/Assets/Blueprints/Actors/BP_AGridPiece.BP_AGridPiece_C|GetCube (Utilities|Array|Get(acopy) (Variables|Default|GetGrid) _index)) 0 "/Game/StarterContent/Materials/M_CobbleStone_Pebble.M_CobbleStone_Pebble")
  (Variables|/Game/Assets/Blueprints/Actors/AC_GridPieceStats.AC_GridPieceStats_C|SetIsPainted (Variables|/Game/Assets/Blueprints/Actors/BP_AGridPiece.BP_AGridPiece_C|GetStats (Utilities|Array|Get(acopy) (Variables|Default|GetGrid) _index)) true))

(fn RowColumntoIndex
  (params (Row :type Integer) (Column :type Integer))
  (return (+ (* Row (Variables|Default|GetNumColumns)) Column)))

(fn AddObstacle
  (params (Row :type Integer) (Column :type Integer))
  (Development|PrintString (Utilities|String|ToString(Integer) Row))
  (Development|PrintString (Utilities|String|ToString(Integer) Column))
  (Utilities|FlowControl|Sequence
    (:then_0
      (LocalVariables|Setez_row Row)
      (LocalVariables|Setez_column Column))
    (:then_1
      (if (or (or (< (LocalVariables|Getez_row) 0) (< (LocalVariables|Getez_column) 0)) (or (>= (LocalVariables|Getez_row) (Variables|Default|GetNumRows)) (>= (LocalVariables|Getez_column) (Variables|Default|GetNumColumns))))
        (return)))
    (:then_2
      (bind _index (CallFunction|RowColumntoIndex Row Column))
      (Variables|/Script/Engine.PrimitiveComponent|SetbGenerateOverlapEvents (Variables|/Game/Assets/Blueprints/Actors/BP_AGridPiece.BP_AGridPiece_C|GetWall (Utilities|Array|Get(acopy) (Variables|Default|GetGrid) _index)) true)
      (Rendering|SetVisibility (Variables|/Game/Assets/Blueprints/Actors/BP_AGridPiece.BP_AGridPiece_C|GetWall (Utilities|Array|Get(acopy) (Variables|Default|GetGrid) _index)) true false))))

(fn GetOpenSpots
  (params (Row :type Integer) (Column :type Integer) (Direction :type Vector))
  (bind (_x _y) (Math|Vector|BreakVector Direction))
  (LocalVariables|SetRowPos Row)
  (LocalVariables|SetColPos Column)
  (LocalVariables|SetRowDir (Math|Float|Truncate _x))
  (LocalVariables|SetColumnDir (Math|Float|Truncate _y))
  (Utilities|FlowControl|Sequence
    (:then_0
      ;[1 1 1] if spot opposite direction is in bounds and painted
      (bind _ispainted (CallFunction|IsPainted (- (LocalVariables|GetRowPos) (LocalVariables|GetRowDir)) (- (LocalVariables|GetColPos) (LocalVariables|GetColumnDir))))
      (if (and (and (>= (- (LocalVariables|GetRowPos) (LocalVariables|GetRowDir)) 0) (>= (- (LocalVariables|GetColPos) (LocalVariables|GetColumnDir)) 0)) _ispainted)
        (return 0)))
    (:then_1
      (while (and (and (> (LocalVariables|GetRowPos) 0) (< (LocalVariables|GetRowPos) (Variables|Default|GetNumRows))) (and (> (LocalVariables|GetColPos) 0) (< (LocalVariables|GetColPos) (Variables|Default|GetNumColumns))))
        (LocalVariables|SetNumSpots (+ (LocalVariables|GetNumSpots) 1))
        (bind _output_get (LocalVariables|SetColPos (+ (LocalVariables|GetColPos) (LocalVariables|GetColumnDir))))
        (bind _output_get_2 (LocalVariables|SetRowPos (+ (LocalVariables|GetRowPos) (LocalVariables|GetRowDir))))
        (bind _ispainted_2 (CallFunction|IsPainted _output_get_2 _output_get))
        (if _ispainted_2
          (return (LocalVariables|GetNumSpots))))
      (return (LocalVariables|GetNumSpots)))))

(fn IsPainted
  (params (Row :type Integer) (Column :type Integer))
  (bind _index (CallFunction|RowColumntoIndex Row Column))
  (Utilities|FlowControl|Sequence
    (:then_0
      (if (or (or (>= Row (Variables|Default|GetNumRows)) (>= Column (Variables|Default|GetNumColumns))) (or (< Row 0) (< Column 0)))
        (return true)))
    (:then_1
      (return (Variables|/Game/Assets/Blueprints/Actors/AC_GridPieceStats.AC_GridPieceStats_C|GetIsPainted (Variables|/Game/Assets/Blueprints/Actors/BP_AGridPiece.BP_AGridPiece_C|GetStats (Utilities|Array|Get(acopy) (Variables|Default|GetGrid) _index)))))))